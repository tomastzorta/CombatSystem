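; Low-tier melee enemy character that plays a climb-up intro montage on spawn and shows its health bar widget while targeted.
; Weapon collision component traces the weapon mesh and applies point damage from a stats component value to actors that can receive it.
; Toggling combat snaps the weapon between its hand and default attach sockets.
; Death extends the parent logic by simulating weapon physics and disabling movement.
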(event `self.ReceiveBeginPlay`
  (`parent.ReceiveBeginPlay`)
  (`/Game/CombatSystem/Blueprints/Components/BAC_CollisionComponent.SetCollisionMesh` (`self.BAC_MainWeaponCollisionComponent`) (`self.WeaponMesh`))
  (bind _returnvalue (`|CreateWidget` "/Game/CombatSystem/UI/WBP_HealthBar.WBP_HealthBar_C" (`GameplayStatics.GetPlayerController` 0) (`self.BAC_StatsComponent`)))
  (`WidgetComponent.SetWidget` (`self.HealthBar`) _returnvalue)
  (`self.PlayAnimMontage` "/Game/CombatSystem/Blueprints/AI/AI_Types/Low_Enemy/Animations/Intro/AM_LowEnemy_IntroClimbUp.AM_LowEnemy_IntroClimbUp"))

(event `self.OnTargeted`
  (params (bIsTargeted :type Boolean))
  (`parent.OnTargeted` bIsTargeted)
  (`SceneComponent.SetVisibility` (`self.HealthBar`) bIsTargeted false))

(event `self.BAC_MainWeaponCollisionComponent.OnHit`
  (params (HitResult :type "HitResult Structure"))
  (bind (_bblockinghit _binitialoverlap _time _distance _location _impactpoint _normal _impactnormal _physmat _hitactor) (`GameplayStatics.BreakHitResult` HitResult))
  (bind _returnvalue (message `/Game/CombatSystem/Blueprints/Interfaces/BPI_Combat.Can Receive Damage` _hitactor))
  (if _returnvalue
    (`GameplayStatics.ApplyPointDamage` _hitactor (`/Game/CombatSystem/Blueprints/Components/BAC_StatsComponent.GetCurrentStatValue` (`self.BAC_StatsComponent`) "NewEnumerator4") (`self.GetActorForwardVector`) HitResult (`self.GetController`) self "/Game/CombatSystem/Blueprints/DamageTypes/BPDT_AttackDamageType.BPDT_AttackDamageType_C")))

(event `Simulate Weapon Physics`
  (bind _weaponmesh (`self.WeaponMesh`))
  (`PrimitiveComponent.SetCollisionProfileName` _weaponmesh "PhysicsActor" true)
  (`PrimitiveComponent.SetSimulatePhysics` _weaponmesh true))

(event `self.PerformDeath`
  (`parent.PerformDeath`)
  (`self.Simulate Weapon Physics`)
  (`CharacterMovementComponent.SetMovementMode` (`self.CharacterMovement`) "MOVE_None" 0))

(event `self.AC_CombatComponent.OnCombatToggled`
  (params (bIsCombatEnabled :type Boolean))
  (`SceneComponent.K2_AttachToComponent` (`self.WeaponMesh`) (`self.Mesh`) (select `bool` bIsCombatEnabled :`false` (`self.Weapon Attach Socket Name`) :`true` (`self.Weapon Hand Attach Socket Name`)) "SnapToTarget" "SnapToTarget" "SnapToTarget" true))

(fn `UserConstructionScript`
  (`parent.UserConstructionScript`))