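; BP_MobEnemy is a melee AI enemy that extends a parent AI class with a weapon mesh and a health bar widget.
; The health bar reads the stats component and shows only while the enemy is targeted.
; The collision component traces the weapon mesh and applies stat-based point damage to actors that can receive it.
; Combat toggles move the weapon between hand and carry sockets, and death turns it into a physics object.
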(event `self.ReceiveBeginPlay`
  (`parent.ReceiveBeginPlay`)
  (`/Game/CombatSystem/Blueprints/Components/BAC_CollisionComponent.SetCollisionMesh` (`self.BAC_MainWeaponCollisionComponent`) (`self.Get AI Weapon`))
  (bind _returnvalue (`|CreateWidget` "/Game/CombatSystem/UI/WBP_HealthBar.WBP_HealthBar_C" (`GameplayStatics.GetPlayerController` 0) (`self.BAC_StatsComponent`)))
  (`WidgetComponent.SetWidget` (`self.HealthBar`) _returnvalue))

(event `/Game/CombatSystem/Blueprints/Interfaces/BPI_Targeting.OnTargeted`
  (params (bIsTargeted :type Boolean))
  (`parent.OnTargeted` bIsTargeted)
  (`SceneComponent.SetVisibility` (`self.HealthBar`) bIsTargeted false))

(event `self.BAC_MainWeaponCollisionComponent.OnHit`
  (params (HitResult :type "HitResult Structure"))
  (bind (_bblockinghit _binitialoverlap _time _distance _location _impactpoint _normal _impactnormal _physmat _hitactor) (`GameplayStatics.BreakHitResult` HitResult))
  (bind _returnvalue (message `/Game/CombatSystem/Blueprints/Interfaces/BPI_Combat.Can Receive Damage` _hitactor))
  (if _returnvalue
    (`GameplayStatics.ApplyPointDamage` _hitactor (`/Game/CombatSystem/Blueprints/Components/BAC_StatsComponent.GetCurrentStatValue` (`self.BAC_StatsComponent`) "NewEnumerator4") (`self.GetActorForwardVector`) HitResult (`self.GetController`) self "/Game/CombatSystem/Blueprints/DamageTypes/BPDT_AttackDamageType.BPDT_AttackDamageType_C")))

(event `Simulate Weapon Physics`
  (`PrimitiveComponent.SetCollisionProfileName` (`self.Get AI Weapon`) "PhysicsActor" true)
  (`PrimitiveComponent.SetSimulatePhysics` (`self.Get AI Weapon`) true))

(event `self.PerformDeath`
  (`parent.PerformDeath`)
  (`self.Simulate Weapon Physics`))

(event `self.AC_CombatComponent.OnCombatToggled`
  (params (bIsCombatEnabled :type Boolean))
  (`SceneComponent.K2_AttachToComponent` (`self.Get AI Weapon`) (`self.Mesh`) (select `bool` bIsCombatEnabled :`false` (`self.Weapon Attach Socket Name`) :`true` (`self.Weapon Hand Attach Socket Name`)) "SnapToTarget" "SnapToTarget" "SnapToTarget" true))

(fn `Get AI Weapon`
  (returns (`Return Value` :type "PrimitiveComponent Object Reference"))
  (return (`self.AI Weapon Mesh`)))

(fn `UserConstructionScript`
  (`parent.UserConstructionScript`))