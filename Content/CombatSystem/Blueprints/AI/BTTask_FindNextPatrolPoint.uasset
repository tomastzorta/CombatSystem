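; Behavior tree task that picks the next patrol destination for a BP_MasterAI from its patrol point array.
; It projects the point at the blackboard patrol index onto the navmesh and writes it as the target location, failing if the pawn or point is invalid.
; It then steps the index, ping-ponging between the ends when ShouldAILoopPatrol is set, otherwise staying at the last point.
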(event `self.ReceiveExecuteAI`
  (params (OwnerController :type "AIController Object Reference") (ControlledPawn :type "Pawn Object Reference"))
  (bind _asbp_master_ai (cast `/Game/CombatSystem/Blueprints/AI/BP_MasterAI` ControlledPawn)
    (:`then`
      (set `self.Controlled Master AI` _asbp_master_ai)
      (bind _bwassuccessful (`self.SetAIPathLocation`))
      (if _bwassuccessful
        (if (`self.bShouldMoveBack`)
          (`self.DecrementAIPathIndex`)
          (else
            (`self.IncrementAIPathIndex`)))
        (`self.FinishExecute` true)
        (else
          (`self.FinishExecute` false))))
    (:`CastFailed`
      (`self.FinishExecute` false))))

(fn `DecrementAIPathIndex`
  (locals (L_AIPatrolIndex :type Integer))
  (bind _l_aipatrolindex (`local.L_AIPatrolIndex`))
  (set `local.L_AIPatrolIndex` (- (`BTFunctionLibrary.GetBlackboardValueAsInt` (`self.AIPatrolIndex`)) 1))
  (if (>= _l_aipatrolindex 0)
    (`BTFunctionLibrary.SetBlackboardValueAsInt` (`self.AIPatrolIndex`) _l_aipatrolindex)
    (else
      (set `self.bShouldMoveBack` false)
      (`self.IncrementAIPathIndex`))))

(fn `IncrementAIPathIndex`
  (locals (L_AIPatrolIndex :type Integer))
  (bind _output_get (set `local.L_AIPatrolIndex` (+ (`BTFunctionLibrary.GetBlackboardValueAsInt` (`self.AIPatrolIndex`)) 1)))
  (if (> (`local.L_AIPatrolIndex`) (`KismetArrayLibrary.Array_LastIndex` (`/Game/CombatSystem/Blueprints/AI/BP_MasterAI.AIPatrolPoints` (`self.Controlled Master AI`))))
    (if (`self.bShouldAILoopPatrol`)
      (set `self.bShouldMoveBack` true)
      (`self.DecrementAIPathIndex`))
    (else
      (`BTFunctionLibrary.SetBlackboardValueAsInt` (`self.AIPatrolIndex`) _output_get))))

(fn `SetAIPathLocation`
  (returns (bWasSuccessful :type Boolean))
  (bind _output (`|GetArrayItem` (`/Game/CombatSystem/Blueprints/AI/BP_MasterAI.AIPatrolPoints` (`self.Controlled Master AI`)) (`BTFunctionLibrary.GetBlackboardValueAsInt` (`self.AIPatrolIndex`))))
  (`/Engine/EditorBlueprintResources/StandardMacros.IsValid` _output
    (:`Is Valid`
      (`BTFunctionLibrary.SetBlackboardValueAsVector` (`self.AITargetLocation`) (`NavigationSystemV1.K2_ProjectPointToNavigation` (`Actor.K2_GetActorLocation` _output)))
      (return true))
    (:`Is Not Valid`
      (return false))))