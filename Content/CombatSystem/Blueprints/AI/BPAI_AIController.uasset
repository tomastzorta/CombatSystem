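; AI controller for combat-system enemies that runs the possessed BP_MasterAI pawn's behavior tree and picks its target.
; Perception updates check each sensed actor's stimuli by index, treating 0 as sight and 1 as damage.
; Either sense sets the AITarget blackboard key to actors tagged Character.Player.
; A failed sight stimulus clears the key regardless of which actor was lost, while a failed damage stimulus leaves it untouched.
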(event `self.ReceivePossess`
  (params (PossessedPawn :type "Pawn Object Reference"))
  (bind _asbp_master_ai (cast `/Game/CombatSystem/Blueprints/AI/BP_MasterAI` PossessedPawn))
  (set `self.Master AI` _asbp_master_ai)
  (`self.RunBehaviorTree` (`/Game/CombatSystem/Blueprints/AI/BP_MasterAI.Behaviour Tree` (`self.Master AI`))))

(event `self.AIPerception.OnPerceptionUpdated`
  (params (UpdatedActors :type "Array of Actor Object Reference (by ref)"))
  (`self.UpdateAIPerception` UpdatedActors))

(fn `UpdateAIPerception`
  (params (PerceivedActors :type "Array of Actor Object Reference"))
  (locals (L_PerceivedActor :type "Actor Object Reference") (L_AIStimuli :type "AIStimulus Structure"))
  (for _array_element PerceivedActors
    (set `local.L_PerceivedActor` _array_element)
    (bind _info (`AIPerceptionComponent.GetActorsPerception` (`self.AIPerception`) (`local.L_PerceivedActor`)))
    (for (_array_element_2 _array_index) (`.LastSensedStimuli` (break `ActorPerceptionBlueprintInfo` _info))
      (set `local.L_AIStimuli` _array_element_2)
      (switch `int` _array_index
        (:`0`
          ;[0.01096 0.01161 0.0137] Index 0 = Sight
          (if (`.bSuccessfullySensed` (break `AIStimulus` (`local.L_AIStimuli`)))
            (bind _return_bool (message `/Game/CombatSystem/Blueprints/Interfaces/BPI_GameplayTagsBlueprint.HasMatchingGameplayTagBP` (`local.L_PerceivedActor`) (struct :`TagName` "Character.Player")))
            (if _return_bool
              (`BlackboardComponent.SetValueAsObject` (`self.Blackboard`) "AITarget" (`local.L_PerceivedActor`)))
            (else
              (`BlackboardComponent.SetValueAsObject` (`self.Blackboard`) "AITarget" null))))
        (:`1`
          ;[0.01096 0.01161 0.0137] Index 1 = Damage
          (if (`.bSuccessfullySensed` (break `AIStimulus` (`local.L_AIStimuli`)))
            (bind _return_bool_2 (message `/Game/CombatSystem/Blueprints/Interfaces/BPI_GameplayTagsBlueprint.HasMatchingGameplayTagBP` (`local.L_PerceivedActor`) (struct :`TagName` "Character.Player")))
            (if _return_bool_2
              (`BlackboardComponent.SetValueAsObject` (`self.Blackboard`) "AITarget" (`local.L_PerceivedActor`)))))))))

(fn `UserConstructionScript`)