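; AN_ConsumeEquippedItem is an animation notify that uses up an equipped consumable at a chosen point in an animation.
; It looks up the item in the owner's equipment component by a gameplay tag and casts it to BP_Base_Consumable.
; If the cast succeeds, it calls ConsumeItemUse and then deducts a fixed score penalty through the owner's player metrics component.
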(fn `Received_Notify`
  (params (MeshComp :type "SkeletalMeshComponent Object Reference") (Animation :type "AnimSequenceBase Object Reference") (EventReference :type "AnimNotifyEventReference Structure (by ref)"))
  (returns (ReturnValue :type Boolean))
  (bind _returnvalue (`ActorComponent.GetOwner` MeshComp))
  (bind _asbp_base_consumable (cast `/Game/CombatSystem/Blueprints/Actors/BP_Base_Consumable` (`/Game/CombatSystem/Blueprints/Components/BAC_Equipment_Component.Get Equipped Item By Gameplay Tag` (`Actor.GetComponentByClass` _returnvalue "/Game/CombatSystem/Blueprints/Components/BAC_Equipment_Component.BAC_Equipment_Component_C") (`self.Equipped Item Tag To Consume`))))
  (`/Game/CombatSystem/Blueprints/Actors/BP_Base_Consumable.Consume Item Use` _asbp_base_consumable)
  (`/Game/CombatSystem/Blueprints/Components/BAC_PlayerMetrics_Component.Minus Player Score` (`Actor.GetComponentByClass` _returnvalue "/Game/CombatSystem/Blueprints/Components/BAC_PlayerMetrics_Component.BAC_PlayerMetrics_Component_C") (`KismetMathLibrary.Conv_IntToDouble` 10))
  (return true))