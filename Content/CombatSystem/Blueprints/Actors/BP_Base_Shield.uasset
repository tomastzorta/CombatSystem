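; Base shield actor for the combat system, handling how a shield is equipped on and removed from its owner.
; On equip it caches the owner's combat, state and stats components, binds to combat toggling, and attaches to the hand or attach socket by combat state.
; It registers as the combat component's shield and points weapon collision at its mesh, ignoring the owner.
; Unequipping runs parent logic and clears that registration.
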(fn `OnEquipped`
  (`self.SetIsEquipped` true)
  (`self.AttachActor` (`self.AttachSocketName`))
  (bind _output_get (set `self.Combat Component` (`self.GetComponentByClass` (`self.GetOwner`) "/Game/CombatSystem/Blueprints/Components/BAC_Combat_Component.BAC_Combat_Component_C")))
  (add `/Game/CombatSystem/Blueprints/Components/BAC_Combat_Component.OnCombatToggled` _output_get (`|CreateDelegate` :!event `Toggle Weapon Combat`))
  (set `self.OwnerStateManager` (`self.GetComponentByClass` (`self.GetOwner`) "/Game/CombatSystem/Blueprints/Components/BAC_StateManager_Component.BAC_StateManager_Component_C"))
  (set `self.OwnerStatsManager` (`self.GetComponentByClass` (`self.GetOwner`) "/Game/CombatSystem/Blueprints/Components/BAC_Stats_Component.BAC_Stats_Component_C"))
  (`self.AttachActor` (select `bool` (`/Game/CombatSystem/Blueprints/Components/BAC_Combat_Component.Is Combat Enabled` (`self.Combat Component`)) :`false` (`self.AttachSocketName`) :`true` (`self.HandSocketName`)))
  (`/Game/CombatSystem/Blueprints/Components/BAC_Combat_Component.Set Shield Weapon` (`self.Combat Component`) self)
  (`/Game/CombatSystem/Blueprints/Components/BAC_Collision_Component.SetCollisionMesh` (`self.BAC_MainWeaponCollisionComponent`) (`self.GetItemMesh`))
  (`/Game/CombatSystem/Blueprints/Components/BAC_Collision_Component.AddActorToIgnore` (`self.BAC_MainWeaponCollisionComponent`) (`self.GetOwner`)))

(fn `OnUnequipped`
  (`parent.OnUnequipped`)
  (`/Game/CombatSystem/Blueprints/Components/BAC_Combat_Component.Set Shield Weapon` (`self.Combat Component`) null))

(fn `UserConstructionScript`
  (`parent.UserConstructionScript`))