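; Base Blueprint for a sword-and-shield weapon that adds a shield mesh to the parent weapon's equip and combat behavior.
; The shield static mesh attaches to the owning character's mesh at a hand socket during combat and at a separate attach socket otherwise.
; Equipping places the shield by the current combat state and flags it as equipped on the combat component, and unequipping clears that flag.
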(event `self.Toggle Weapon Combat`
  (params (bEnableCombat :type Boolean))
  (`parent.Toggle Weapon Combat` bEnableCombat)
  (`self.Attach Shield Weapon` (select `bool` bEnableCombat :`false` (`self.Shield Attach Socket Name`) :`true` (`self.Shield Hand Socket Name`))))

(fn `Attach Shield Weapon`
  (params (`Attach Socket Name` :type Name))
  (`SceneComponent.K2_AttachToComponent` (`self.Shield Item Static Mesh`) (`Character.Mesh` (cast `Character` (`self.GetOwner`) :!pure true)) `Attach Socket Name` "KeepRelative" "KeepRelative" "KeepRelative" true))

(fn `OnEquipped`
  (`parent.OnEquipped`)
  (`self.Attach Shield Weapon` (select `bool` (`/Game/CombatSystem/Blueprints/Components/BAC_Combat_Component.Is Combat Enabled` (`self.Combat Component`)) :`false` (`self.Shield Attach Socket Name`) :`true` (`self.Shield Hand Socket Name`)))
  (`/Game/CombatSystem/Blueprints/Components/BAC_Combat_Component.Set Is Shield Equipped On Character` (`self.Combat Component`) true))

(fn `OnUnequipped`
  (`parent.OnUnequipped`)
  (`/Game/CombatSystem/Blueprints/Components/BAC_Combat_Component.Set Is Shield Equipped On Character` (`self.Combat Component`) false))

(fn `UserConstructionScript`
  (`parent.UserConstructionScript`))