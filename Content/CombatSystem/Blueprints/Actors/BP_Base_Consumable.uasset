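; Base Blueprint for equippable consumables with limited uses that change one of the owner's stats, such as a health potion.
; Uses are filled to the maximum on BeginPlay, and using the item asks the owner to play the use montage as a tagged action while any remain.
; A separate ConsumeItemUse event decrements uses, reports the count to the owner and applies the configured change through its BAC_StatsComponent.
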(event `self.ReceiveBeginPlay`
  (`parent.ReceiveBeginPlay`)
  (set `self.Equipped Item Uses` (`self.Equipped Item Max Uses`)))

(event `self.Use Equipped Item`
  (if (> (`self.Equipped Item Uses`) 0)
    (message `/Game/CombatSystem/Blueprints/Interfaces/BPI_Combat.Perform Altered Action` (`self.GetOwner`) (struct :`TagName` "Character.Action.Use Equipped Item") (struct :`TagName` "Character.State.General Action State") (`self.Use Equipped Item Montage`) 1.0 false)))

(event `Consume Item Use`
  (bind _returnvalue (`self.GetOwner`))
  (bind _result (`/Engine/EditorBlueprintResources/StandardMacros.DecrementInt` (`self.Equipped Item Uses`))
    (:`  `
      (message `/Game/CombatSystem/Blueprints/Interfaces/BPI_Combat.Update Health Potion Remaining Uses` _returnvalue _result)
      (`/Game/CombatSystem/Blueprints/Components/BAC_StatsComponent.ModifyCurrentStatValue` (`self.GetComponentByClass` _returnvalue "/Game/CombatSystem/Blueprints/Components/BAC_StatsComponent.BAC_StatsComponent_C") (`self.Stat`) (`self.Changed Value`) (`self.Should Regenerate`)))))

(fn `UserConstructionScript`
  (`parent.UserConstructionScript`))