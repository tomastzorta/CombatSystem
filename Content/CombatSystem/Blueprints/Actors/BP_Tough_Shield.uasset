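; BP_Tough_Shield is a shield actor in the combat system that supplies the animation montages for character actions.
; GetActionMontages switches on a Character.Action gameplay tag and returns the matching montage set for attack variants, dodge, combat enter and exit, or block.
; Enter and exit combat wrap single montages in arrays, while block returns shield-specific animations.
; The event graph holds only disabled stubs, and construction just calls the parent.
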(fn `GetActionMontages`
  (params (`Character Action` :type "GameplayTag Structure"))
  (returns (Montages :type "Array of AnimMontage Object Reference"))
  (`|SwitchGameplayTag` `Character Action`
    (:`Character.Action.Attack.Light Attack`
      (return (`self.LightAttackMontages`)))
    (:`Character.Action.Attack.Heavy Attack`
      (return (`self.HeavyAttackMontages`)))
    (:`Character.Action.Attack.Sprint Attack`
      (return (`self.SprintAttackMontages`)))
    (:`Character.Action.Attack.Charged Attack`
      (return (`self.ChargedAttackMontages`)))
    (:`Character.Action.Attack.Falling Attack`
      (return (`self.FallingAttackMontages`)))
    (:`Character.Action.Dodge`
      (return (`self.DodgeMontages`)))
    (:`Character.Action.Enter Combat`
      (return (`|MakeArray` (`self.Enter Combat`))))
    (:`Character.Action.Exit Combat`
      (return (`|MakeArray` (`self.Exit Combat`))))
    (:`Character.Action.Block`
      (return (`self.Shield Block Animations`)))))

(fn `UserConstructionScript`
  (`parent.UserConstructionScript`))