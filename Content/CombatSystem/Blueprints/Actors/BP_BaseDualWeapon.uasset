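; Base dual-wield weapon actor that adds an off-hand weapon mesh and a right-foot hit source to its parent weapon.
; On equip and combat toggle, the off-hand mesh snaps to a hand or stowed socket on the owning Character's mesh.
; Separate collision components for main weapon, off-hand and right foot are switched by body part and ignore the owner.
; Off-hand and foot hits apply point damage to actors that accept damage messages.
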(event `self.Toggle Combat`
  (params (bEnableCombat :type Boolean))
  (`parent.Toggle Combat` bEnableCombat)
  (`self.AttachOffHandWeapon` (select `bool` bEnableCombat :`false` (`self.Second Weapon Attach Socket`) :`true` (`self.Second Weapon Hand Socket`))))

(event `self.BAC_OffHandWeaponCollisionComponent.OnHit`
  (params (HitResult :type "HitResult Structure"))
  (bind (_bblockinghit _binitialoverlap _time _distance _location _impactpoint _normal _impactnormal _physmat _hitactor) (`GameplayStatics.BreakHitResult` HitResult))
  (bind _returnvalue (message `/Game/CombatSystem/Blueprints/Interfaces/BPI_Combat.Can Receive Damage` _hitactor))
  (if _returnvalue
    (`GameplayStatics.ApplyPointDamage` _hitactor (`self.GetDamage`) (`self.GetActorForwardVector` (`self.GetOwner`)) HitResult (`self.GetInstigatorController`) self)))

(event `self.BAC_RightFootCollisionComponent.OnHit`
  (params (HitResult :type "HitResult Structure"))
  (bind (_bblockinghit _binitialoverlap _time _distance _location _impactpoint _normal _impactnormal _physmat _hitactor) (`GameplayStatics.BreakHitResult` HitResult))
  (bind _returnvalue (message `/Game/CombatSystem/Blueprints/Interfaces/BPI_Combat.Can Receive Damage` _hitactor))
  (if _returnvalue
    (`GameplayStatics.ApplyPointDamage` _hitactor (`self.GetDamage`) (`self.GetActorForwardVector` (`self.GetOwner`)) HitResult (`self.GetInstigatorController`) self)))

(fn `ActivateCollision`
  (params (`Collision Part` :type "/Game/CombatSystem/Blueprints/Enums/E_CollisionPart Enum" :default "NewEnumerator0"))
  (switch `/Game/CombatSystem/Blueprints/Enums/E_CollisionPart` `Collision Part`
    (:`NewEnumerator0`
      (`/Game/CombatSystem/Blueprints/Components/BAC_CollisionComponent.ActivateCollision` (`self.BAC_MainWeaponCollisionComponent`)))
    (:`NewEnumerator1`
      (`/Game/CombatSystem/Blueprints/Components/BAC_CollisionComponent.ActivateCollision` (`self.BAC_OffHandWeaponCollisionComponent`)))
    (:`NewEnumerator2`
      (`/Game/CombatSystem/Blueprints/Components/BAC_CollisionComponent.ActivateCollision` (`self.BAC_RightFootCollisionComponent`)))))

(fn `AttachOffHandWeapon`
  (params (Socket :type Name))
  (`SceneComponent.K2_AttachToComponent` (`self.Off Hand Weapon Mesh`) (`Character.Mesh` (cast `Character` (`self.GetOwner`) :!pure true)) Socket "SnapToTarget" "SnapToTarget" "SnapToTarget" true))

(fn `DeactivateCollision`
  (params (`Collision Part` :type "/Game/CombatSystem/Blueprints/Enums/E_CollisionPart Enum" :default "NewEnumerator0"))
  (switch `/Game/CombatSystem/Blueprints/Enums/E_CollisionPart` `Collision Part`
    (:`NewEnumerator0`
      (`/Game/CombatSystem/Blueprints/Components/BAC_CollisionComponent.DeactivateCollision` (`self.BAC_MainWeaponCollisionComponent`)))
    (:`NewEnumerator1`
      (`/Game/CombatSystem/Blueprints/Components/BAC_CollisionComponent.DeactivateCollision` (`self.BAC_OffHandWeaponCollisionComponent`)))
    (:`NewEnumerator2`
      (`/Game/CombatSystem/Blueprints/Components/BAC_CollisionComponent.DeactivateCollision` (`self.BAC_RightFootCollisionComponent`)))))

(fn `OnEquipped`
  (`parent.OnEquipped`)
  (`/Game/CombatSystem/Blueprints/Components/BAC_CollisionComponent.SetCollisionMesh` (`self.BAC_OffHandWeaponCollisionComponent`) (`self.Off Hand Weapon Mesh`))
  (`/Game/CombatSystem/Blueprints/Components/BAC_CollisionComponent.SetCollisionMesh` (`self.BAC_RightFootCollisionComponent`) (`Character.Mesh` (cast `Character` (`self.GetOwner`) :!pure true)))
  (`self.AttachOffHandWeapon` (select `bool` (`/Game/CombatSystem/Blueprints/Components/BAC_CombatComponent.Is Combat Enabled` (`self.Combat Component`)) :`false` (`self.Second Weapon Attach Socket`) :`true` (`self.Second Weapon Hand Socket`)))
  (`/Game/CombatSystem/Blueprints/Components/BAC_CollisionComponent.AddActorToIgnore` (`self.BAC_MainWeaponCollisionComponent`) (`self.GetOwner`))
  (`/Game/CombatSystem/Blueprints/Components/BAC_CollisionComponent.AddActorToIgnore` (`self.BAC_OffHandWeaponCollisionComponent`) (`self.GetOwner`))
  (`/Game/CombatSystem/Blueprints/Components/BAC_CollisionComponent.AddActorToIgnore` (`self.BAC_RightFootCollisionComponent`) (`self.GetOwner`)))

(fn `UserConstructionScript`
  (`parent.UserConstructionScript`))