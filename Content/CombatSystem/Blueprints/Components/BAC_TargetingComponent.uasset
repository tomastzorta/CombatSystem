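; Actor component that gives its owning Character toggleable lock-on targeting for combat.
; Lock-on sphere-traces along the camera's forward vector for a BPI_Targeting actor and notifies it when targeted.
; Each tick it interpolates control pitch and yaw toward the target, releasing lock when CanTargetActor fails.
; Lock changes switch between orient-to-camera and the default rotation mode, based on combat state and movement speed mode.
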(event `self.ReceiveBeginPlay`
  (bind _ascharacter (cast `Character` (`self.GetOwner`)))
  (set `self.Owner Character` _ascharacter)
  (set `self.Owner Controller` (`Pawn.GetController` (`self.Owner Character`)))
  (set `self.Followed Camera` (`Actor.GetComponentByClass` (`self.Owner Character`) "/Script/Engine.CameraComponent")))

(event `Toggle Lock On`
  (if (not (`self.IsTargeting`))
    (`self.Enable Lock On`)
    (else
      (`self.Disable Lock On`))))

(event `Enable Lock On`
  (bind (_return_value _found_target) (`self.Find Lock On Target`))
  (if (and _return_value (`self.Can Target Actor` _found_target))
    (`self.Set Target Actor` _found_target)
    (`self.SetIsTargeting` true)
    (`self.UpdateRotationMode`)))

(event `Disable Lock On`
  (`self.SetIsTargeting` false)
  (`self.Set Target Actor` null)
  (`self.UpdateRotationMode`))

(event `self.ReceiveTick`
  (params (DeltaSeconds :type "Float (single-precision)"))
  (`parent.ReceiveTick` DeltaSeconds)
  (if (`self.bIsTargeting`)
    (`self.Update Targeting Control Rotation`)))

(fn `Can Target Actor`
  (params (`In Target Actor` :type "Actor Object Reference"))
  (returns (ReturnValue :type Boolean))
  (`/Engine/EditorBlueprintResources/StandardMacros.IsValid` `In Target Actor`
    (:`Is Valid`
      (bind _return_value (message `/Game/CombatSystem/Blueprints/Interfaces/BPI_Targeting.CanBeTargeted` `In Target Actor`))
      (return (and _return_value (< (`Actor.GetDistanceTo` (`self.GetOwner`) (`self.Target Actor`)) (`self.Targeting Distance`)))))
    (:`Is Not Valid`
      (return false))))

(fn `Find Lock On Target`
  (returns (`Return Value` :type Boolean) (`Found Target` :type "Actor Object Reference"))
  (bind (_outhit _returnvalue) (`KismetSystemLibrary.SphereTraceSingleForObjects` (`Actor.K2_GetActorLocation` (`self.GetOwner`)) (+ (* (`SceneComponent.GetForwardVector` (`self.Followed Camera`)) (`self.Targeting Distance`)) (`Actor.K2_GetActorLocation` (`self.GetOwner`))) (`self.Targeting Radius`) (`self.Target Object Types`) false (`|MakeArray` (`self.GetOwner`))))
  (bind (_bblockinghit _binitialoverlap _time _distance _location _impactpoint _normal _impactnormal _physmat _hitactor) (`GameplayStatics.BreakHitResult` _outhit))
  (if (and _returnvalue (`KismetSystemLibrary.IsValid` _hitactor))
    (if (`KismetSystemLibrary.DoesImplementInterface` _hitactor "/Game/CombatSystem/Blueprints/Interfaces/BPI_Targeting.BPI_Targeting_C")
      (return true _hitactor)
      (else
        _)))
  (return false null))

(fn `Get Character Rotation Mode`
  (returns (`Return Value` :type "/Game/CombatSystem/Blueprints/Enums/E_RotationMode Enum"))
  (return (`self.Current Rotation Mode`)))

(fn `Get Target Actor`
  (returns (`Return Value` :type "Actor Object Reference"))
  (return (`self.Target Actor`)))

(fn `IsTargeting`
  (returns (`Return Value` :type Boolean))
  (return (`self.bIsTargeting`)))

(fn `Set Character Rotation Mode`
  (params (`New Rotation Mode` :type "/Game/CombatSystem/Blueprints/Enums/E_RotationMode Enum" :default "NewEnumerator0"))
  (bind _owner_character (`self.Owner Character`))
  (bind _charactermovement (`Character.CharacterMovement` _owner_character))
  (bind _output_get (set `self.Current Rotation Mode` `New Rotation Mode`))
  (switch `/Game/CombatSystem/Blueprints/Enums/E_RotationMode` _output_get
    (:`NewEnumerator0`
      (set `Pawn.bUseControllerRotationYaw` false _owner_character)
      (set `CharacterMovementComponent.bUseControllerDesiredRotation` true _charactermovement)
      (set `CharacterMovementComponent.bOrientRotationToMovement` false _charactermovement))
    (:`NewEnumerator1`
      (set `Pawn.bUseControllerRotationYaw` false _owner_character)
      (set `CharacterMovementComponent.bUseControllerDesiredRotation` false _charactermovement)
      (set `CharacterMovementComponent.bOrientRotationToMovement` true _charactermovement))))

(fn `Set Target Actor`
  (params (`New Target Actor` :type "Actor Object Reference"))
  (set `self.Target Actor` `New Target Actor`))

(fn `SetIsTargeting`
  (params (bEnableTargeting :type Boolean))
  (set `self.bIsTargeting` bEnableTargeting)
  (bind _target_actor (`self.Target Actor`)
    (:`then`
      (message `/Game/CombatSystem/Blueprints/Interfaces/BPI_Targeting.OnTargeted` _target_actor (`local.bEnableTargeting`)))
    (:`else`)))

(fn `Update Targeting Control Rotation`
  (bind _returnvalue (`Actor.K2_GetActorRotation` (`self.Owner Controller`)))
  (bind (_returnvalue_roll _returnvalue_pitch _returnvalue_yaw) (`KismetMathLibrary.BreakRotator` (`KismetMathLibrary.RInterpTo` _returnvalue (`KismetMathLibrary.FindLookAtRotation` (`Actor.K2_GetActorLocation` (`self.GetOwner`)) (- (`Actor.K2_GetActorLocation` (`self.Target Actor`)) (0.0 0.0 100.0))) (`GameplayStatics.GetWorldDeltaSeconds`) (`self.Target Rotation Interp Speed`))))
  (if (and (`KismetSystemLibrary.IsValid` (`self.Target Actor`)) (`KismetSystemLibrary.IsValid` (`self.Owner Controller`)))
    (if (`self.Can Target Actor` (`self.Target Actor`))
      (`Controller.SetControlRotation` (`self.Owner Controller`) (`KismetMathLibrary.MakeRotator` (.roll _returnvalue) _returnvalue_pitch _returnvalue_yaw))
      (else
        (`self.Disable Lock On`)))))

(fn `UpdateRotationMode`
  (`/Engine/EditorBlueprintResources/StandardMacros.IsValid` (`self.Owner Combat Component`)
    (:`Is Valid`
      (bind _return_value (message `/Game/CombatSystem/Blueprints/Interfaces/BPI_Combat.Get Movement Speed Mode` (`self.Owner Character`)))
      (`self.Set Character Rotation Mode` (select `bool` (and (`/Game/CombatSystem/Blueprints/Components/BAC_CombatComponent.Is Combat Enabled` (`self.Owner Combat Component`)) (`|EnumInequality` _return_value "NewEnumerator2") (`self.IsTargeting`)) :`false` (`self.Default Rotation Mode`) :`true` "NewEnumerator0")))
    (:`Is Not Valid`
      (set `self.Owner Combat Component` (`Actor.GetComponentByClass` (`self.Owner Character`) "/Game/CombatSystem/Blueprints/Components/BAC_CombatComponent.BAC_CombatComponent_C")))))