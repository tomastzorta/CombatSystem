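; Combat component that holds a character's equipped main weapon and shield, plus its combat, blocking and attack state.
; Setting a main weapon unequips and destroys the previous one, while setting a shield only stores the reference.
; Combat and blocking setters broadcast their new state through event dispatchers, with blocking firing only on change.
; ResetAttack clears the attack count and saved-attack flag; the event graph is empty.
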(fn `Get Equipped Shield Weapon`
  (returns (`Return Value` :type "/Game/CombatSystem/Blueprints/Actors/BP_Base_Weapon Object Reference"))
  (return (`self. `)))

(fn `Get Main weapon`
  (returns (`Return Value` :type "/Game/CombatSystem/Blueprints/Actors/BP_Base_Weapon Object Reference"))
  (return (`self.Main Character Weapon`)))

(fn `Is Character Blocking`
  (returns (`Return Value` :type Boolean))
  (return (`self.bIsCharacterBlocking`)))

(fn `Is Combat Enabled`
  (returns (`Return value` :type Boolean))
  (return (`self.bCombatEnabled`)))

(fn `Reset Attack`
  (set `self.Attack Count` 0)
  (set `self.bIsAttackSaved` false))

(fn `Set Character Blocking State`
  (params (bEnableCharacterBlocking :type Boolean))
  (if (!= bEnableCharacterBlocking (`self.bIsCharacterBlocking`))
    (bind _output_get (set `self.bIsCharacterBlocking` (`local.bEnableCharacterBlocking`)))
    (`self.On Character Blocking Set` _output_get)))

(fn `Set Combat Enabled`
  (params (bEnableCombat :type Boolean))
  (bind _output_get (set `self.bCombatEnabled` bEnableCombat))
  (`self.OnCombatToggled` _output_get))

(fn `Set Main Weapon`
  (params (`New Weapon` :type "/Game/CombatSystem/Blueprints/Actors/BP_Base_Weapon Object Reference"))
  (bind _main_character_weapon (`self.Main Character Weapon`))
  (`|ExecutionSequence`
    (:`then_0`
      (`/Engine/EditorBlueprintResources/StandardMacros.IsValid` _main_character_weapon
        (:`Is Valid`
          (`/Game/CombatSystem/Blueprints/Actors/BP_Base_Equipabble.OnUnequipped` _main_character_weapon)
          (`Actor.K2_DestroyActor` (`self.Main Character Weapon`)))))
    (:`then_1`
      (set `self.Main Character Weapon` (`local.New Weapon`)))))

(fn `Set Shield Weapon`
  (params (`Shield Weapon` :type "/Game/CombatSystem/Blueprints/Actors/BP_Base_Weapon Object Reference"))
  (set `self. ` `Shield Weapon`))