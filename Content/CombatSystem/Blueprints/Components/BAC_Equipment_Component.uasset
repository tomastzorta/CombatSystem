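; Equipment component for the combat system that spawns and tracks the items its owning actor has equipped.
; InitialiseEquipment spawns each valid StartingEquipment class at the owner's transform, sets owner and instigator, stores it in EquippedItems and calls OnEquipped.
; Items are looked up by gameplay tag, either to use the first match and report success or to return it.
; BeginPlay and Tick are unused, so initialisation relies on an external call.
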(fn `Get Equipped Item By Gameplay Tag`
  (params (`Item Gameplay Tag` :type "GameplayTag Structure"))
  (returns (`Returned Item` :type "/Game/CombatSystem/Blueprints/Actors/BP_Base_Equipabble Object Reference"))
  (for _array_element (`self.Equipped Items`)
    (`/Engine/EditorBlueprintResources/StandardMacros.IsValid` _array_element
      (:`Is Valid`
        (bind _return_bool (`/Game/CombatSystem/Blueprints/Actors/BP_Base_Equipabble.HasMatchingGameplayTagBP` _array_element `Item Gameplay Tag`))
        (if _return_bool
          (return _array_element)))))
  (return null))

(fn `Initialise Equipment`
  (bind _returnvalue (`self.GetOwner`))
  (for _array_element (`self.Starting Equipment`)
    (if (`KismetSystemLibrary.IsValidClass` _array_element)
      (bind _returnvalue_2 (`|SpawnActorFromClass` _array_element (`Actor.GetTransform` _returnvalue) "Undefined" "MultiplyWithRoot" _returnvalue (cast `Pawn` _returnvalue :!pure true)))
      (`KismetArrayLibrary.Array_AddUnique` (`self.Equipped Items`) _returnvalue_2)
      (`/Game/CombatSystem/Blueprints/Actors/BP_Base_Equipabble.OnEquipped` _returnvalue_2)))
  (return))

(fn `Perform Action From Equipped Item`
  (params (`Equipped Item To Check` :type "GameplayTag Structure"))
  (returns (bWasItSuccessful :type Boolean))
  (for _array_element (`self.Equipped Items`)
    (`/Engine/EditorBlueprintResources/StandardMacros.IsValid` _array_element
      (:`Is Valid`
        (bind _return_bool (`/Game/CombatSystem/Blueprints/Actors/BP_Base_Equipabble.HasMatchingGameplayTagBP` _array_element `Equipped Item To Check`))
        (if _return_bool
          (`/Game/CombatSystem/Blueprints/Actors/BP_Base_Equipabble.Use Equipped Item` _array_element)
          (return true)))))
  (return false))