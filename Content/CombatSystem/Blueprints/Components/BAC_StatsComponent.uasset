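; Actor component for the combat system that holds an actor's stats as base, max and current values in maps keyed by stat type.
; Current-value changes notify through an update call, and modifications clamp between zero and max with optional regeneration.
; Only stamina regenerates, through a retriggerable delay and a looping timer that stops when full.
; Damage lowers health and, at zero, changes the owner's state through its state manager component.
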(event `StartRegen`
  (params (`Stat Type` :type "/Game/CombatSystem/Blueprints/Enums/E_Stats Enum" :default "NewEnumerator0"))
  (switch `/Game/CombatSystem/Blueprints/Enums/E_Stats` `Stat Type`
    (:`NewEnumerator2`
      (`KismetSystemLibrary.K2_ClearTimer` null "RegenerateStamina")
      (`KismetSystemLibrary.RetriggerableDelay` 1.5)
      (`KismetSystemLibrary.K2_SetTimer` null "RegenerateStamina" 0.1 true))))

(fn `GetBaseStatValue`
  (params (Stat :type "/Game/CombatSystem/Blueprints/Enums/E_Stats Enum" :default "NewEnumerator0"))
  (returns (`Base Value` :type "Float (double-precision)"))
  (return (break `/Game/CombatSystem/Blueprints/Structs/F_BaseStat` (`BlueprintMapLibrary.Map_Find` (`self.Base Stats`) Stat))))

(fn `GetCurrentStatValue`
  (params (Stat :type "/Game/CombatSystem/Blueprints/Enums/E_Stats Enum" :default "NewEnumerator0"))
  (returns (Value :type "Float (double-precision)"))
  (return (`BlueprintMapLibrary.Map_Find` (`self.Current Stats`) Stat)))

(fn `GetMaxStatValue`
  (params (Stat :type "/Game/CombatSystem/Blueprints/Enums/E_Stats Enum" :default "NewEnumerator0"))
  (returns (`Max Value` :type "Float (double-precision)"))
  (return (`.MaxValue_4_5EFC4E504D9C9267454576A29F644FBD` (break `/Game/CombatSystem/Blueprints/Structs/F_BaseStat` (`BlueprintMapLibrary.Map_Find` (`self.Base Stats`) Stat)))))

(fn `InitialiseStats`
  (bind _keys (`BlueprintMapLibrary.Map_Keys` (`self.Base Stats`)))
  (for _array_element _keys
    (`self.SetCurrentStatValue` _array_element (break `/Game/CombatSystem/Blueprints/Structs/F_BaseStat` (`BlueprintMapLibrary.Map_Find` (`self.Base Stats`) _array_element)))))

(fn `ModifyCurrentStatValue`
  (params (Stat :type "/Game/CombatSystem/Blueprints/Enums/E_Stats Enum" :default "NewEnumerator0") (Value :type "Float (double-precision)") (bShouldRegenerate :type Boolean :default true))
  (locals (L_Value :type "Float (double-precision)"))
  (bind _stat (`local.Stat`))
  (if (!= Value 0.0)
    (bind _output_get (set `local.L_Value` (+ (`self.GetCurrentStatValue` (`local.Stat`)) (`local.Value`))))
    (bind _output_get_2 (set `local.L_Value` (`KismetMathLibrary.FClamp` _output_get 0.0 (`self.GetMaxStatValue` (`local.Stat`)))))
    (`self.SetCurrentStatValue` _stat _output_get_2)
    (if (`local.bShouldRegenerate`)
      (`self.StartRegen` _stat))))

(fn `RegenerateStamina`
  (`self.SetCurrentStatValue` "NewEnumerator2" (`KismetMathLibrary.FClamp` (+ (`self.GetCurrentStatValue` "NewEnumerator2") (`self.StaminaRegenerateRate`)) 0.0 (`self.GetMaxStatValue` "NewEnumerator2")))
  (if (>= (`self.GetCurrentStatValue` "NewEnumerator2") (`self.GetMaxStatValue` "NewEnumerator2"))
    (`KismetSystemLibrary.K2_ClearTimer` null "RegenerateStamina")))

(fn `SetBaseStatValue`
  (params (Stat :type "/Game/CombatSystem/Blueprints/Enums/E_Stats Enum" :default "NewEnumerator0") (Value :type "Float (double-precision)"))
  (bind _structout (setmembers `/Game/CombatSystem/Blueprints/Structs/F_BaseStat` :`StructRef` (`BlueprintMapLibrary.Map_Find` (`self.Base Stats`) Stat) :`Base Value` Value))
  (`BlueprintMapLibrary.Map_Add` (`self.Base Stats`) (`local.Stat`) _structout))

(fn `SetCurrentStatValue`
  (params (Stat :type "/Game/CombatSystem/Blueprints/Enums/E_Stats Enum" :default "NewEnumerator0") (Value :type "Float (double-precision)"))
  (`BlueprintMapLibrary.Map_Add` (`self.Current Stats`) Stat Value)
  (`self.OnCurrentStatValueUpdated` (`local.Stat`) (`local.Value`)))

(fn `SetMaxStatValue`
  (params (Stat :type "/Game/CombatSystem/Blueprints/Enums/E_Stats Enum" :default "NewEnumerator0") (Value :type "Float (double-precision)"))
  (bind _structout (setmembers `/Game/CombatSystem/Blueprints/Structs/F_BaseStat` :`StructRef` (`BlueprintMapLibrary.Map_Find` (`self.Base Stats`) Stat) :`Max Value` Value))
  (`BlueprintMapLibrary.Map_Add` (`self.Base Stats`) (`local.Stat`) _structout))

(fn `TakeDamage`
  (params (InDamage :type "Float (double-precision)"))
  (`self.ModifyCurrentStatValue` "NewEnumerator1" (* (`local.InDamage`) -1.0))
  (if (<= (`self.GetCurrentStatValue` "NewEnumerator1") 0.0)
    (`/Game/CombatSystem/Blueprints/Components/BAC_StateManagerComponent.SetState` (`Actor.GetComponentByClass` (`self.GetOwner`) "/Game/CombatSystem/Blueprints/Components/BAC_StateManagerComponent.BAC_StateManagerComponent_C") "NewEnumerator4")))