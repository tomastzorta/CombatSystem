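; Combat collision component that detects hits along an assigned mesh during an activation window and reports them through OnHit.
; While enabled, each Tick runs a multi-sphere object trace between the mesh's start and end sockets, skipping ignored actors.
; Hits are filtered by gameplay tags, ignored classes and an already-hit list, which is cleared on activation so each actor registers once per activation.
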(event `SetCollisionMesh`
  (params (CollisionMeshComponent :type "PrimitiveComponent Object Reference"))
  ;[1 1 1] Set Collision Mesh
  (set `self.CollisionMeshComponent` CollisionMeshComponent))

(event `ActivateCollision`
  ;[1 1 1] Enable Collision
  (`self.ClearHitActors`)
  (set `self.bIsCollisionEnabled` true))

(event `self.ReceiveTick`
  (params (DeltaSeconds :type "Float (single-precision)"))
  (if (`self.bIsCollisionEnabled`)
    (`self.CollisionTrace`)))

(event `DeactivateCollision`
  ;[1 1 1] Disable Collision
  (set `self.bIsCollisionEnabled` false))

(event `ClearHitActors`
  ;[1 1 1] Clear Hit Actors
  (`KismetArrayLibrary.Array_Clear` (`self.AlreadyHitActors`)))

(event `CollisionTrace`
  (bind _collisionmeshcomponent (`self.CollisionMeshComponent`))
  ;[1 1 1] Collision Trace
  (bind _outhits (`KismetSystemLibrary.SphereTraceMultiForObjects` (`SceneComponent.GetSocketLocation` _collisionmeshcomponent (`self.Start Socket Name`)) (`SceneComponent.GetSocketLocation` _collisionmeshcomponent (`self.EndSocketName`)) (`self.Trace Radius`) (`self.Collision Object Types`) false (`self.Actors to Ignore`) (`self.Draw Debug Type`)))
  (for _array_element _outhits
    (bind _output_get (set `self.Last Hit` _array_element))
    (bind (_bblockinghit _binitialoverlap _time _distance _location _impactpoint _normal _impactnormal _physmat _hitactor) (`GameplayStatics.BreakHitResult` _output_get))
    (if (`self.Can Hit Actor` _hitactor)
      (bind _output_get_2 (set `self.Hit Actor` _hitactor))
      (`KismetArrayLibrary.Array_Add` (`self.AlreadyHitActors`) _output_get_2)
      (`self.OnHit` (`self.Last Hit`)))))

(fn `AddActorToIgnore`
  (params (HitActor :type "Actor Object Reference (by ref)"))
  (`KismetArrayLibrary.Array_AddUnique` (`self.Actors to Ignore`) HitActor))

(fn `Can Hit Actor`
  (params (ActorHit :type "Actor Object Reference (by ref)"))
  (returns (ReturnValue :type Boolean))
  (bind _return_tag (message `/Game/CombatSystem/Blueprints/Interfaces/BPI_GameplayTagsBlueprint.GetOwnedGameplayTags` ActorHit))
  (return (and (not (`BlueprintGameplayTagLibrary.HasAnyTags` _return_tag (`self.Gameplay Tags To Ignore`) true)) (not (`KismetArrayLibrary.Array_Contains` (`self.AlreadyHitActors`) ActorHit)) (not (`KismetArrayLibrary.Array_Contains` (`self.Ignored Actors`) (`GameplayStatics.GetObjectClass` (`local.ActorHit`)))))))

(fn `GetActorsToIgnore`
  (returns (`Actors to Ignore` :type "Array of Actor Object Reference"))
  (return (`self.Actors to Ignore`)))

(fn `GetAlreadyHitActors`
  (returns (AlreadyHitActors :type "Array of Actor Object Reference"))
  (return (`self.AlreadyHitActors`)))

(fn `GetCollisionMeshComponent`
  (returns (CollisionMeshComponent :type "PrimitiveComponent Object Reference"))
  (return (`self.CollisionMeshComponent`)))

(fn `GetLastHit`
  (returns (`Last Hit` :type "HitResult Structure"))
  (return (`self.Last Hit`)))

(fn `IsCollisionEnabled`
  (returns (bIsCollisionEnabled :type Boolean))
  (return (`self.bIsCollisionEnabled`)))

(fn `RemoveActorToIgnore`
  (params (ItemToRemove :type "Actor Object Reference (by ref)"))
  (`KismetArrayLibrary.Array_RemoveItem` (`self.Actors to Ignore`) ItemToRemove))