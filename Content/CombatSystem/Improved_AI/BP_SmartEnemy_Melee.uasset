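; BP_SmartEnemy_Melee is a melee AI enemy that implements attack, equip and unequip weapon events through animation montages.
; Equipping spawns a BP_Tough_Sword on a montage notify and snaps it to the right-hand socket, while unequipping moves it to the hip socket.
; Both notifies update the wielding flag.
; Each montage fires its matching end callback whether completed or interrupted.
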(event `/Game/CombatSystem/Improved_AI/AI_Functionality/Smart_Interfaces/BPI_SmartAI.AI Attack`
  (`|PlayMontage` (`self.Mesh`) "/Game/Assets/Free_Assets/Animations/LightSword/LightAttack/AI_Test_Attack.AI_Test_Attack"
    (:`OnCompleted`
      _)
    (:`OnInterrupted`
      _))
  (`self.On AI Attack End`))

(event `/Game/CombatSystem/Improved_AI/AI_Functionality/Smart_Interfaces/BPI_SmartAI.AI Equip Weapon`
  (bind _notifyname (`|PlayMontage` (`self.Mesh`) "/Game/Assets/Free_Assets/Animations/LightSword/Equip/AM_AITest_Unsheathe.AM_AITest_Unsheathe")
    (:`OnCompleted`
      (`self.On AI Unsheathe Weapon` :!label _label))
    (:`OnInterrupted`
      (goto _label))
    (:`OnNotifyBegin`
      (switch `name` _notifyname
        (:`Unsheathe Weapon`
          (bind _returnvalue (`|SpawnActorFromClass` "/Game/CombatSystem/Blueprints/Actors/BP_Tough_Sword.BP_Tough_Sword_C" (`self.GetTransform`) "Undefined" "MultiplyWithRoot" null null))
          (bind _output_get (set `self.AI Weapon` _returnvalue))
          (`self.K2_AttachToComponent` _output_get (`self.Mesh`) "RightWeaponSocket" "SnapToTarget" "SnapToTarget" "SnapToTarget" true)
          (set `self.bIs AI Weilding Weapon` true))))))

(event `/Game/CombatSystem/Improved_AI/AI_Functionality/Smart_Interfaces/BPI_SmartAI.AI Unequip Weapon`
  (bind _notifyname (`|PlayMontage` (`self.Mesh`) "/Game/Assets/Free_Assets/Animations/LightSword/Equip/AM_AITest_Sheathe.AM_AITest_Sheathe")
    (:`OnCompleted`
      (`self.On AI Sheathe Weapon` :!label _label_2))
    (:`OnInterrupted`
      (goto _label_2))
    (:`OnNotifyBegin`
      (switch `name` _notifyname
        (:`Sheathe Weapon`
          (`self.K2_AttachToComponent` (`self.AI Weapon`) (`self.Mesh`) "SwordHipAttachSocket" "SnapToTarget" "SnapToTarget" "SnapToTarget" true)
          (set `self.bIs AI Weilding Weapon` false))))))

(fn `UserConstructionScript`
  (`parent.UserConstructionScript`))