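; BP_SmartEnemy_Ranged is a smart enemy character that attacks at range with blockable projectiles.
; On BeginPlay it spawns a sword-and-shield weapon and attaches it to the right-hand socket.
; AIAttack plays a throw montage whose notify fires a projectile through BACUniversalAttacks from the weapon toward the AI controller's target, signalling attack end on completion or interruption.
; It also supplies attack and defend radii and maps movement states to walk speeds.
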(event `self.ReceiveBeginPlay`
  (`parent.ReceiveBeginPlay`)
  (`/Game/CombatSystem/Improved_AI/AI_Functionality/Smart_Interfaces/BPI_SmartAI.AI Equip Weapon`))

(event `/Game/CombatSystem/Improved_AI/AI_Functionality/Smart_Interfaces/BPI_SmartAI.AI Equip Weapon`
  (bind _returnvalue (`|SpawnActorFromClass` "/Game/CombatSystem/Blueprints/Actors/BP_Tough_SwordAndShield.BP_Tough_SwordAndShield_C" (`KismetMathLibrary.MakeTransform` (0.0 0.0 0.0)) "Undefined" "MultiplyWithRoot" null null))
  (bind _output_get (set `self.AI Weapon` _returnvalue))
  (`self.K2_AttachToComponent` _output_get (`self.Mesh`) "RightWeaponSocket" "SnapToTarget" "SnapToTarget" "SnapToTarget" true)
  (set `self.bIs AI Weilding Weapon` true)
  (`self.On AI Unsheathe Weapon`))

(event `/Game/CombatSystem/Improved_AI/AI_Functionality/Smart_Interfaces/BPI_SmartAI.AI Attack`
  (set `self.bIs AI Attacking` true)
  (bind _notifyname (`|PlayMontage` (`self.Mesh`) "/Game/AM_AI_Throw_Test.AM_AI_Throw_Test")
    (:`OnCompleted`
      (`self.On AI Attack End` :!label _label)
      (set `self.bIs AI Attacking` false))
    (:`OnInterrupted`
      (goto _label))
    (:`OnNotifyBegin`
      (switch `name` _notifyname
        (:`Throw`
          (bind _asaic_smart_enemy_base (cast `/Game/CombatSystem/Improved_AI/AI_Functionality/Controllers/AIC_SmartEnemy_Base` (`AIBlueprintHelperLibrary.GetAIController` self)))
          (bind _ai_attack_target (`/Game/CombatSystem/Improved_AI/AI_Functionality/Controllers/AIC_SmartEnemy_Base.AI Attack Target` _asaic_smart_enemy_base)
            (:`then`
              (`/Game/CombatSystem/Improved_AI/Player/Components/BAC_Universal_Attacks.Regular: Projectile` (`self.BAC_Universal_Attacks`) (`self.K2_GetActorLocation` (`self.AI Weapon`)) (`self.K2_GetActorLocation` _ai_attack_target) (make `/Game/CombatSystem/Improved_AI/Improved_DamageSystem/S_DamageInfo` 15.0 "NewEnumerator2" "NewEnumerator0" false true)))
            (:`else`)))))))

(fn `Change AI Movement Speed`
  (params (`AI Movement Speed` :type "/Game/CombatSystem/Improved_AI/AI_Functionality/Enums/E_AI_MovementSpeeds Enum" :default "NewEnumerator0"))
  (returns (`Movement Speed Value` :type "Float (double-precision)"))
  (set `CharacterMovementComponent.MaxWalkSpeed` (select `/Game/CombatSystem/Improved_AI/AI_Functionality/Enums/E_AI_MovementSpeeds` `AI Movement Speed` :`NewEnumerator1` 100.0 :`NewEnumerator2` 300.0 :`NewEnumerator3` 500.0 :!type "Float (single-precision)") (`self.CharacterMovement`))
  (return 0.0))

(fn `Get AI Range`
  (returns (`AI Attack Radius` :type "Float (double-precision)") (`AI Defend Radius` :type "Float (double-precision)"))
  (return 600.0 600.0))

(fn `UserConstructionScript`
  (`parent.UserConstructionScript`))