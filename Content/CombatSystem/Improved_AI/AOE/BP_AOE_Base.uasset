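; BP_AOE_Base is a base area-of-effect actor for the combat system that detects pawns within a radius.
; TriggerAOE, optionally run shortly after BeginPlay, performs a sphere overlap at the actor's location.
; The overlap can skip the instigator and draw a debug sphere.
; Each hit actor is broadcast through OnAOECollisionWithActor, leaving the actual effect outside this graph.
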(event `self.ReceiveBeginPlay`
  (if (`self.bShouldTriggerOnGameStart`)
    (`KismetSystemLibrary.Delay` 0.1)
    (`self.Trigger AOE`)))

(event `AOE Spawn Shape: Sphere`
  (if (`self.bShouldDrawDebugSphere`)
    (`KismetSystemLibrary.DrawDebugSphere` (`self.K2_GetActorLocation`) (`self.AOE Radius`) 12 (struct :`R` 1.0 :`B` 0.802695 :`A` 1.0) 1.0 1.0))
  (bind _outactors (`KismetSystemLibrary.SphereOverlapActors` (`self.K2_GetActorLocation`) (`self.AOE Radius`) (`|MakeArray` "ObjectTypeQuery3" :!type "EObjectTypeQuery Enum") null (`|MakeArray` (select `bool` (`self.bShouldIgnoreAOEInstigator`) :`true` (`self.Instigator`) :!type "Actor Object Reference"))))
  (for _array_element _outactors
    (`self.On AOE Collision With Actor` _array_element)))

(event `Trigger AOE`
  (`self.AOE Spawn Shape: Sphere`))

(fn `UserConstructionScript`)