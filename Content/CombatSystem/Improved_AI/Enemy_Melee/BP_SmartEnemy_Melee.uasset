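; Melee variant of the smart enemy AI, supplying its sword-fighting attacks, weapon handling and combat ranges.
; Attack events for ground smash, short range, long-range jump and spin pass montage and damage info, including block/parry rules where set, to BACUniversalAttacks.
; Equip and unequip montage notifies spawn a sword into the hand or move it to the hip, and montage end fires delegates.
; A helper predicts target position from horizontal velocity.
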(event `AI Melee Attack: Ground Smash`
  (params (`AI Attack Target` :type "Actor Object Reference"))
  ;[0.7812 0.02936 0] AI Attacking Logic
  (`/Game/CombatSystem/Improved_AI/Player/Components/BAC_Universal_Attacks.Universal Attack: Ground Smash` (`self.BAC_Universal_Attacks`) (make `/Game/CombatSystem/Improved_AI/Structures/S_AttackInfo` `AI Attack Target` "/Game/Animations/Melee/AM_AI_Melee_Ability_GroundSmash.AM_AI_Melee_Ability_GroundSmash" (make `/Game/CombatSystem/Improved_AI/Improved_DamageSystem/S_DamageInfo` 25.0 "NewEnumerator3")) 300.0))

(event `AI Melee Attack: Short Range`
  (params (`AI Attack Target` :type "Actor Object Reference"))
  ;[0.7812 0.02936 0] AI Attacking Logic
  (`/Game/CombatSystem/Improved_AI/Player/Components/BAC_Universal_Attacks.Actor Melee Attack: Short Range` (`self.BAC_Universal_Attacks`) (make `/Game/CombatSystem/Improved_AI/Structures/S_AttackInfo` `AI Attack Target` "/Game/Assets/Free_Assets/Animations/LightSword/LightAttack/AI_Test_Attack.AI_Test_Attack" (make `/Game/CombatSystem/Improved_AI/Improved_DamageSystem/S_DamageInfo` 10.0 "NewEnumerator1" "NewEnumerator1" false true true)) 20.0 200.0))

(event `self.ReceiveBeginPlay`
  (`parent.ReceiveBeginPlay`))

(event `AI Melee Attack: Long Range`
  (params (`AI Attack Target` :type "Actor Object Reference"))
  ;[0.7812 0.02936 0] AI Attacking Logic
  (`/Game/CombatSystem/Improved_AI/Player/Components/BAC_Universal_Attacks.Actor Melee Attack: Long Range` (`self.BAC_Universal_Attacks`) (make `/Game/CombatSystem/Improved_AI/Structures/S_AttackInfo` `AI Attack Target` "/Game/Assets/Free_Assets/Animations/LightSword/ChargeAttack/AM_AI_Melee_JumpAttack.AM_AI_Melee_JumpAttack" (make `/Game/CombatSystem/Improved_AI/Improved_DamageSystem/S_DamageInfo` 20.0 "NewEnumerator1" "NewEnumerator2" false true true))))

(event `/Game/CombatSystem/Improved_AI/AI_Functionality/Smart_Interfaces/BPI_SmartAI.AI Equip Weapon`
  ;[0.4688 0.03602 0] AI Equip And Unequip Weapon
  (bind _notifyname (`|PlayMontage` (`self.Mesh`) "/Game/Assets/Free_Assets/Animations/LightSword/Equip/AM_AITest_Unsheathe.AM_AITest_Unsheathe")
    (:`OnCompleted`
      (`self.On AI Unsheathe Weapon` :!label _label))
    (:`OnInterrupted`
      (goto _label))
    (:`OnNotifyBegin`
      (switch `name` _notifyname
        (:`Unsheathe Weapon`
          (bind _returnvalue (`|SpawnActorFromClass` "/Game/CombatSystem/Blueprints/Actors/BP_Tough_Sword.BP_Tough_Sword_C" (`self.GetTransform`) "Undefined" "MultiplyWithRoot" null null))
          (bind _output_get (set `self.AI Weapon` _returnvalue))
          (`self.K2_AttachToComponent` _output_get (`self.Mesh`) "RightWeaponSocket" "SnapToTarget" "SnapToTarget" "SnapToTarget" true)
          (set `self.bIs AI Weilding Weapon` true))))))

(event `AI Melee Attack: Spin Attack`
  (params (`AI Attack Target` :type "Actor Object Reference"))
  ;[0.7812 0.02936 0] AI Attacking Logic
  (`/Game/CombatSystem/Improved_AI/Player/Components/BAC_Universal_Attacks.Actor Melee Attack: Spin Attack` (`self.BAC_Universal_Attacks`) (make `/Game/CombatSystem/Improved_AI/Structures/S_AttackInfo` `AI Attack Target` "/Game/Animations/Melee/AM_AI_Melee_SpinAttack.AM_AI_Melee_SpinAttack" (make `/Game/CombatSystem/Improved_AI/Improved_DamageSystem/S_DamageInfo` 10.0 "NewEnumerator1" "NewEnumerator1" false true))))

(event `/Game/CombatSystem/Improved_AI/AI_Functionality/Smart_Interfaces/BPI_SmartAI.AI Unequip Weapon`
  ;[0.4688 0.03602 0] AI Equip And Unequip Weapon
  (bind _notifyname (`|PlayMontage` (`self.Mesh`) "/Game/Assets/Free_Assets/Animations/LightSword/Equip/AM_AITest_Sheathe.AM_AITest_Sheathe")
    (:`OnCompleted`
      (`self.On AI Sheathe Weapon` :!label _label_2))
    (:`OnInterrupted`
      (goto _label_2))
    (:`OnNotifyBegin`
      (switch `name` _notifyname
        (:`Sheathe Weapon`
          (`self.K2_AttachToComponent` (`self.AI Weapon`) (`self.Mesh`) "SwordHipAttachSocket" "SnapToTarget" "SnapToTarget" "SnapToTarget" true)
          (set `self.bIs AI Weilding Weapon` false))))))

(fn `Get AI Range`
  (returns (`AI Attack Radius` :type "Float (double-precision)") (`AI Defend Radius` :type "Float (double-precision)"))
  (return 200.0 400.0))

(fn `Predict AI Attack Target Position`
  (params (`AI Attack Target` :type "Actor Object Reference") (`Future Predict Time` :type "Float (double-precision)" :default 1.0))
  (returns (`AI Attack Target Predicted Location` :type "Vector Structure"))
  (return (+ (`self.K2_GetActorLocation` (`local.AI Attack Target`)) (* (* (`self.GetVelocity` `AI Attack Target`) (1.0 1.0 0.0)) `Future Predict Time`))))

(fn `UserConstructionScript`
  (`parent.UserConstructionScript`))