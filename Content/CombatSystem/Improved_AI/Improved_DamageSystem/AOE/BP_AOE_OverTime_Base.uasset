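; Base area-of-effect Blueprint for effects that act over a duration, extending its parent's TriggerAOE event.
; After calling the parent logic, TriggerAOE starts a looping timer at the effect tick interval, provided that interval is positive.
; It also starts a one-shot timer for the AOE duration; the events both timers fire are not defined in this graph.
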(event `self.Trigger AOE`
  (`parent.Trigger AOE`)
  (`|ExecutionSequence`
    (:`then_0`
      (if (> (`self.AOE Effect Tick Interval`) 0.0)
        (`KismetSystemLibrary.K2_SetTimerDelegate` (`|CreateDelegate` :!event `AOE Spawn Shape: Sphere`) (`self.AOE Effect Tick Interval`) true)))
    (:`then_1`
      (`KismetSystemLibrary.K2_SetTimerDelegate` (`|CreateDelegate` :!event `K2_DestroyActor`) (`self.AOE Duration`)))))

(fn `UserConstructionScript`
  (`parent.UserConstructionScript`))