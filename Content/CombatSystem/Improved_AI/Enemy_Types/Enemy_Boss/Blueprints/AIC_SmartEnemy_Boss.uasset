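; AI controller for the smart enemy boss, which puts the boss health bar on the player's HUD when the boss enters the attacking state.
; Its Set AI State: Attacking override runs the parent logic, then adds the pawn's health bar widget to the target's HUD placeholder.
; A DoOnce gate prevents repeat adds and resets when the target is not a BP_NewCombatCharacter.
; Other active behavior defers to the parent controller.
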(fn `AI Lost Sight`
  (params (`Lost Actor` :type "Actor Object Reference"))
  (`parent.AI Lost Sight` `Lost Actor`))

(fn `Set AI State: Attacking`
  (params (`AI Attack Target` :type "Actor Object Reference") (bUseLastKnownAiTarget :type Boolean))
  (`parent.Set AI State: Attacking` `AI Attack Target` bUseLastKnownAiTarget)
  (`/Engine/EditorBlueprintResources/StandardMacros.DoOnce` false :!label _label
    (:`Completed`
      (bind _asbp_new_combat_character (cast `/Game/CombatSystem/Player/BP_NewCombatCharacter` `AI Attack Target`)
        (:`then`
          (bind _asbp_smart_enemy_boss (cast `/Game/CombatSystem/Improved_AI/Enemy_Types/Enemy_Boss/Blueprints/BP_Smart_Enemy_Boss` (`self.K2_GetPawn`)))
          (`VerticalBox.AddChildToVerticalBox` (`/Game/CombatSystem/Improved_AI/Widgets/WBP_Player_HUD.VB_BossHPPlaceholder` (`/Game/CombatSystem/Player/BP_NewCombatCharacter.Player HUD` _asbp_new_combat_character)) (`/Game/CombatSystem/Improved_AI/Enemy_Types/Enemy_Boss/Blueprints/BP_Smart_Enemy_Boss.Boss Healthbar Widget` _asbp_smart_enemy_boss)))
        (:`CastFailed`
          (goto _label :!via `Reset`))))))

(fn `UserConstructionScript`
  (`parent.UserConstructionScript`))