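; Smart enemy mage AI character that fights with projectile, barrage and ground smash attacks and can heal itself over time.
; Attack events pass montage and damage info to the universal attacks component, while overrides supply movement speeds and attack/defend ranges.
; Healing plays a montage and spawns a heal AOE at a line trace hit, restoring a fraction of max health on self-collision until the montage ends.
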(event `AI Mage Attack: Ground Smash`
  (params (`AI Attack Target` :type "Actor Object Reference"))
  ;[0.7999 0.8475 1] Attacks
  (`/Game/CombatSystem/Improved_AI/Improved_DamageSystem/BAC_Universal_Attacks.Universal Attack: Ground Smash` (`self.BAC_Universal_Attacks`) (make `/Game/CombatSystem/Improved_AI/Improved_DamageSystem/Structures/S_AttackInfo` `AI Attack Target` "/Game/CombatSystem/Improved_AI/Enemy_Types/Enemy_Mage/Animations/Montages/AM_Mage_Ability_GroundSmash.AM_Mage_Ability_GroundSmash" (make `/Game/CombatSystem/Improved_AI/Improved_DamageSystem/Structures/S_DamageInfo` 25.0 "NewEnumerator3")) 300.0))

(event `AI Mage Attack: Base`
  (params (`AI Attack Target` :type "Actor Object Reference"))
  ;[0.7999 0.8475 1] Attacks
  (`/Game/CombatSystem/Improved_AI/Improved_DamageSystem/BAC_Universal_Attacks.Actor Mage Attack: Simple Projectile` (`self.BAC_Universal_Attacks`) (make `/Game/CombatSystem/Improved_AI/Improved_DamageSystem/Structures/S_AttackInfo` `AI Attack Target` "/Game/CombatSystem/Improved_AI/Enemy_Types/Enemy_Mage/Animations/Montages/AM_Mage_RangedAttack.AM_Mage_RangedAttack" (make `/Game/CombatSystem/Improved_AI/Improved_DamageSystem/Structures/S_DamageInfo` 10.0 "NewEnumerator2" "NewEnumerator1"))))

(event `AI Mage Attack: Barrage`
  (params (`AI Attack Target` :type "Actor Object Reference"))
  ;[0.7999 0.8475 1] Attacks
  (`/Game/CombatSystem/Improved_AI/Improved_DamageSystem/BAC_Universal_Attacks.Actor Mage Attack: Barrage` (`self.BAC_Universal_Attacks`) (make `/Game/CombatSystem/Improved_AI/Improved_DamageSystem/Structures/S_AttackInfo` `AI Attack Target` "/Game/CombatSystem/Improved_AI/Enemy_Types/Enemy_Mage/Animations/Montages/AM_Mage_RangedBarrage.AM_Mage_RangedBarrage" (make `/Game/CombatSystem/Improved_AI/Improved_DamageSystem/Structures/S_DamageInfo` 5.0 "NewEnumerator2" "NewEnumerator1"))))

(event `Mage Magic: Enter Heal Self Over Time`
  (bind _returnvalue (`self.K2_GetActorLocation`))
  ;[0.7999 0.8475 1] AI Mage Magic: Heal Self
  (`|PlayMontage` (`self.Mesh`) "/Game/CombatSystem/Improved_AI/Enemy_Types/Enemy_Mage/Animations/Montages/AM_Mage_Ability_Heal.AM_Mage_Ability_Heal"
    (:`then`
      (bind (_outhit _returnvalue_2) (`KismetSystemLibrary.LineTraceSingle` _returnvalue (* _returnvalue (0.0 0.0 -1000.0)) "TraceTypeQuery1"))
      (if _returnvalue_2
        (bind _returnvalue_3 (`|SpawnActorFromClass` "/Game/CombatSystem/Improved_AI/Improved_DamageSystem/AOE/BP_AOE_Heal.BP_AOE_Heal_C" (`KismetMathLibrary.MakeTransform` (`.Location` (`GameplayStatics.BreakHitResult` _outhit))) "Undefined" "MultiplyWithRoot" null 1.0 3.0 false false true null))
        (bind _output_get (set `self.AI Mage Heal Effect` _returnvalue_3))
        (add `/Game/CombatSystem/Improved_AI/Improved_DamageSystem/AOE/BP_AOE_Base.On AOE Collision With Actor` _output_get (delegate `On AOE Collision With Actor_Event`))
        (else
          (`self.StopAnimMontage` null))))
    (:`OnCompleted`
      (`self.Mage Magic: Exit Heal Self Over Time` :!label _label))
    (:`OnInterrupted`
      (goto _label))))

(event `On AOE Collision With Actor_Event`
  (params (Actor :type "Actor Object Reference"))
  ;[0.7999 0.8475 1] AI Mage Magic: Heal Self
  (if (== Actor self)
    (`self.Heal Self` (* (`/Game/CombatSystem/Improved_AI/Improved_DamageSystem/BAC_DamageSystem.Actor Max Health` (`self.BAC_DamageSystem`)) 0.08))))

(event `Mage Magic: Exit Heal Self Over Time`
  ;[0.7999 0.8475 1] AI Mage Magic: Heal Self
  (`self.On AI Magic Heal Exit`)
  (bind _ai_mage_heal_effect (`self.AI Mage Heal Effect`)
    (:`then`
      (`self.K2_DestroyActor` _ai_mage_heal_effect))
    (:`else`)))

(fn `Change AI Movement Speed`
  (params (`AI Movement Speed` :type "/Game/CombatSystem/Improved_AI/AI_Functionality/Enums/E_AI_MovementSpeeds Enum" :default "NewEnumerator0"))
  (returns (`Movement Speed Value` :type "Float (double-precision)"))
  (return (select `/Game/CombatSystem/Improved_AI/AI_Functionality/Enums/E_AI_MovementSpeeds` `AI Movement Speed` :`NewEnumerator1` 150.0 :`NewEnumerator2` 250.0 :`NewEnumerator3` 400.0)))

(fn `Get AI Range`
  (returns (`AI Attack Radius` :type "Float (double-precision)") (`AI Defend Radius` :type "Float (double-precision)"))
  (return 500.0 700.0))

(fn `UserConstructionScript`
  (`parent.UserConstructionScript`))