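; Boss enemy character Blueprint that extends a parent AI with a weapon and an on-screen health bar.
; BeginPlay creates the bar from the stats component, showing it while a player target is set and the boss is alive.
; Left and right weapon collision hits apply stat-based point damage to actors that can receive it.
; Combat toggles move the weapon between sockets, and death enables weapon physics and hides the bar.
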(event `Toggle Boss Health Bar`
  (params (bIsVisible :type Boolean))
  (bind _boss_health_bar_ui (`self.Boss Health Bar UI`)
    (:`then`
      (`Widget.SetVisibility` _boss_health_bar_ui (select `bool` (and bIsVisible (not (`/Game/CombatSystem/Blueprints/Components/BAC_StateManager_Component.IsCurrentStateEqualToAny` (`self.BAC_StateManagerComponent`) (struct :`GameplayTags` (struct :`(TagName` "Character.State.Dead")))))) :`false` "Hidden" :`true` "Visible" :!type "ESlateVisibility Enum")))
    (:`else`)))

(event `self.ReceiveBeginPlay`
  (`parent.ReceiveBeginPlay`)
  (`/Game/CombatSystem/Blueprints/Components/BAC_Collision_Component.SetCollisionMesh` (`self.BAC_RightWeaponCollisionComponent`) (`self.WeaponMesh`))
  (bind _returnvalue (`|CreateWidget` "/Game/CombatSystem/UI/WBP_BossHealthBar.WBP_BossHealthBar_C" (`GameplayStatics.GetPlayerController` 0)))
  (bind _output_get (set `self.Boss Health Bar UI` _returnvalue))
  (`/Game/CombatSystem/UI/WBP_BossHealthBar.Initialise` _output_get (`self.BAC_StatsComponent`))
  (`UserWidget.AddToViewport` (`self.Boss Health Bar UI`) 0))

(event `self.OnTargeted`
  (params (bIsTargeted :type Boolean))
  (`parent.OnTargeted` bIsTargeted))

(event `self.BAC_RightWeaponCollisionComponent.OnHit`
  (params (HitResult :type "HitResult Structure"))
  (`self.Hit Event` HitResult))

(event `Hit Event`
  (params (`Hit Result` :type "HitResult Structure"))
  (bind (_bblockinghit _binitialoverlap _time _distance _location _impactpoint _normal _impactnormal _physmat _hitactor) (`GameplayStatics.BreakHitResult` `Hit Result`))
  (bind _returnvalue (message `/Game/CombatSystem/Blueprints/Interfaces/BPI_Combat.Can Receive Damage` _hitactor))
  (if _returnvalue
    (`GameplayStatics.ApplyPointDamage` _hitactor (`/Game/CombatSystem/Blueprints/Components/BAC_Stats_Component.GetCurrentStatValue` (`self.BAC_StatsComponent`) "NewEnumerator4") (`self.GetActorForwardVector`) `Hit Result` (`self.GetController`) self "/Game/CombatSystem/Blueprints/DamageTypes/BPDT_AttackDamageType.BPDT_AttackDamageType_C")))

(event `self.BAC_LeftWeaponCollisionComponent.OnHit`
  (params (HitResult :type "HitResult Structure"))
  (`self.Hit Event` HitResult))

(event `Simulate Weapon Physics`
  (bind _weaponmesh (`self.WeaponMesh`))
  (`PrimitiveComponent.SetCollisionProfileName` _weaponmesh "PhysicsActor" true)
  (`PrimitiveComponent.SetSimulatePhysics` _weaponmesh true))

(event `self.PerformDeath`
  (`parent.PerformDeath`)
  (`self.Simulate Weapon Physics`)
  (`self.Toggle Boss Health Bar` false))

(event `self.AC_CombatComponent.OnCombatToggled`
  (params (bIsCombatEnabled :type Boolean))
  (`SceneComponent.K2_AttachToComponent` (`self.WeaponMesh`) (`self.Mesh`) (select `bool` bIsCombatEnabled :`false` (`self.Weapon Attach Socket Name`) :`true` (`self.Weapon Hand Attach Socket Name`)) "SnapToTarget" "SnapToTarget" "SnapToTarget" true))

(event `self.OnPlayerTargetSet`
  (params (`New Target` :type "Actor Object Reference"))
  (`parent.OnPlayerTargetSet` `New Target`)
  (`self.Toggle Boss Health Bar` (`KismetSystemLibrary.IsValid` `New Target`)))

(fn `UserConstructionScript`
  (`parent.UserConstructionScript`))