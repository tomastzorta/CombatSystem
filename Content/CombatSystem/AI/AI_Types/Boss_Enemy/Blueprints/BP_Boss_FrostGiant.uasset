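; Frost Giant boss enemy Blueprint, a thin child that relies on its parent class for core behavior.
; On BeginPlay it runs the parent logic, then points the right and left weapon collision components at its mesh.
; It then starts the intro loop montage; the Tick and overlap events are disabled stubs.
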(event `self.ReceiveBeginPlay`
  (`parent.ReceiveBeginPlay`)
  (`/Game/CombatSystem/Blueprints/Components/BAC_CollisionComponent.SetCollisionMesh` (`self.BAC_RightWeaponCollisionComponent`) (`self.Mesh`))
  (`/Game/CombatSystem/Blueprints/Components/BAC_CollisionComponent.SetCollisionMesh` (`self.BAC_LeftWeaponCollisionComponent`) (`self.Mesh`))
  (`self.PlayAnimMontage` "/Game/CombatSystem/AI/AI_Types/Boss_Enemy/Animations/Intro/AM_Boss_FrostGiant_IntroLoop.AM_Boss_FrostGiant_IntroLoop"))

(fn `UserConstructionScript`
  (`parent.UserConstructionScript`))